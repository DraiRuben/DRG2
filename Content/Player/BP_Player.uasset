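; Player Blueprint that lets the player dig and build in chunked voxel terrain.
; Attack and Interact inputs each line-trace from the camera, convert the hit to a chunk-local block position, and call ModifyVoxel recursively on the hit Chunk.
; Attack nudges the hit into the surface to carve Air in a small radius.
; Interact offsets the block along the normal to place Dirt, only if the hit is not too close to the player.
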(event `EnhancedInput|/Game/Inputs/IA_Attack`
  (params (ActionValue :type Boolean) (ElapsedSeconds :type "Float (double-precision)") (TriggeredSeconds :type "Float (double-precision)") (InputAction :type "InputAction Object Reference" :default "/Game/Inputs/IA_Attack.IA_Attack"))
  (bind _camera (`self.Camera`))
  (bind _returnvalue (`SceneComponent.K2_GetComponentLocation` _camera))
  (:`Started`
    (bind (_outhit _returnvalue_2) (`KismetSystemLibrary.LineTraceSingle` _returnvalue (+ _returnvalue (* (`SceneComponent.GetForwardVector` _camera) 800.0)) "TraceTypeQuery2"))
    (if _returnvalue_2
      (bind (_bblockinghit _binitialoverlap _time _distance _location _impactpoint _normal _impactnormal _physmat _hitactor) (`GameplayStatics.BreakHitResult` _outhit))
      (bind _aschunk (cast `Chunk` _hitactor))
      (`Chunk.ModifyVoxel` _aschunk (`VoxelFunctionLibrary.WorldToLocalBlockPosition` (- _location _normal) (make `IntVector` 32 32 384)) "Air" 2.0 true))))

(event `EnhancedInput|/Game/Inputs/IA_Interact`
  (params (ActionValue :type Boolean) (ElapsedSeconds :type "Float (double-precision)") (TriggeredSeconds :type "Float (double-precision)") (InputAction :type "InputAction Object Reference" :default "/Game/Inputs/IA_Interact.IA_Interact"))
  (bind _camera (`self.Camera`))
  (bind _returnvalue (`SceneComponent.K2_GetComponentLocation` _camera))
  (:`Started`
    (bind (_outhit _returnvalue_2) (`KismetSystemLibrary.LineTraceSingle` _returnvalue (+ _returnvalue (* (`SceneComponent.GetForwardVector` _camera) 800.0)) "TraceTypeQuery2"))
    (if _returnvalue_2
      (bind (_bblockinghit _binitialoverlap _time _distance _location _impactpoint _normal _impactnormal _physmat _hitactor) (`GameplayStatics.BreakHitResult` _outhit))
      (if (> (`KismetMathLibrary.Vector_Distance` _location (`self.K2_GetActorLocation`)) 100.0)
        (bind _aschunk (cast `Chunk` _hitactor))
        (`Chunk.ModifyVoxel` _aschunk (`KismetMathLibrary.FTruncVector` (+ _normal (`VoxelFunctionLibrary.WorldToLocalBlockPosition` (- _location _normal) (make `IntVector` 32 32 384)))) "Dirt" 1.9 true)))))

(fn `UserConstructionScript`)